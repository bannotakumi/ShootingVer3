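; Configurable decal actor that projects a material with per-instance tiling, gradient, height, roughness and parallax occlusion settings.
; The Construction Script sets sort order and arrow visibility, then creates a dynamic material instance from the chosen decal material.
; It copies exposed values into scalar parameters, turns boolean switches into 0/1 scalars, and assigns the instance to the decal.
; The event graph holds no logic.
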(event EventBeginPlay)

(event Collision|EventActorBeginOverlap
  (params (OtherActor :type Actor%20Object%20Reference)))

(event EventTick
  (params (DeltaSeconds :type Float%20%28single-precision%29)))

(fn ConstructionScript
  (Utilities|FlowControl|Sequence
    (:then_0
      ;[1 1 1] BASE CONFIG
      (Class|DecalComponent|SetSortOrder (Variables|Default|GetDecal) (Variables|Default|GetSortOrder))
      (Rendering|SetVisibility (Variables|Default|GetArrow) (Variables|Default|GetShow%20Projection%20Direction) false))
    (:then_1
      (bind _returnvalue (Rendering|Material|CreateDynamicMaterialInstance (Variables|Default|GetDecalMaterial) "None" "None" :!class /Script/Engine.KismetMaterialLibrary))
      (Rendering|Material|SetScalarParameterValue _returnvalue "UV Tile U" (Variables|Material|GetUV%20Tile%20U) :!class /Script/Engine.MaterialInstanceDynamic)
      (Rendering|Material|SetScalarParameterValue _returnvalue "UV Tile V" (Variables|Material|GetUV%20Tile%20V) :!class /Script/Engine.MaterialInstanceDynamic)
      (Rendering|Material|SetScalarParameterValue _returnvalue "Gradient Radius" (Variables|Material|GetGradient%20Radius) :!class /Script/Engine.MaterialInstanceDynamic)
      (Rendering|Material|SetScalarParameterValue _returnvalue "Gradient Density" (Variables|Material|GetGradient%20Density) :!class /Script/Engine.MaterialInstanceDynamic)
      (Rendering|Material|SetScalarParameterValue _returnvalue "Height Clamp" (Variables|Material|GetHeight%20Clamp) :!class /Script/Engine.MaterialInstanceDynamic)
      (Rendering|Material|SetScalarParameterValue _returnvalue "Roughness Multiplier" (Variables|Material|GetRoughness%20Multiplier) :!class /Script/Engine.MaterialInstanceDynamic)
      (Rendering|Material|SetScalarParameterValue _returnvalue "Opacity Edge Threshold" (Variables|Material|GetOpacity%20Edge%20Threshold) :!class /Script/Engine.MaterialInstanceDynamic)
      (Rendering|Material|SetScalarParameterValue _returnvalue "Dither Multiplier" (Variables|ParallaxOcclusionMapping|GetDither%20Multiplier) :!class /Script/Engine.MaterialInstanceDynamic)
      (Rendering|Material|SetScalarParameterValue _returnvalue "Max Steps" (Variables|ParallaxOcclusionMapping|GetMax%20Steps) :!class /Script/Engine.MaterialInstanceDynamic)
      (Rendering|Material|SetScalarParameterValue _returnvalue "Min Steps" (Variables|ParallaxOcclusionMapping|GetMin%20Steps) :!class /Script/Engine.MaterialInstanceDynamic)
      (Rendering|Material|SetScalarParameterValue _returnvalue "POM Height" (Variables|ParallaxOcclusionMapping|GetPOM%20Height) :!class /Script/Engine.MaterialInstanceDynamic))
    (:then_2
      (if (Variables|Default|GetUse%20Material%20Alpha)
        (Rendering|Material|SetScalarParameterValue _returnvalue "Use Material Alpha" 1.0 :!class /Script/Engine.MaterialInstanceDynamic)
        (else
          (Rendering|Material|SetScalarParameterValue _returnvalue "Use Material Alpha" 0.0 :!class /Script/Engine.MaterialInstanceDynamic)))
      (if (Variables|Material|GetUse%20Radial%20+%20Height)
        (Rendering|Material|SetScalarParameterValue _returnvalue "Use Radial + Height" 1.0 :!class /Script/Engine.MaterialInstanceDynamic)
        (else
          (Rendering|Material|SetScalarParameterValue _returnvalue "Use Radial + Height" 0.0 :!class /Script/Engine.MaterialInstanceDynamic)))
      (if (Variables|Material|GetUse%20POM)
        (Rendering|Material|SetScalarParameterValue _returnvalue "Use POM" 1.0 :!class /Script/Engine.MaterialInstanceDynamic)
        (else
          (Rendering|Material|SetScalarParameterValue _returnvalue "Use POM" 0.0 :!class /Script/Engine.MaterialInstanceDynamic)))
      (if (Variables|Material|GetInvert%20Roughness)
        (Rendering|Material|SetScalarParameterValue _returnvalue "Invert Roughness" 1.0 :!class /Script/Engine.MaterialInstanceDynamic)
        (else
          (Rendering|Material|SetScalarParameterValue _returnvalue "Invert Roughness" 0.0 :!class /Script/Engine.MaterialInstanceDynamic)))
      (if (Variables|Material|GetInvert%20Height)
        (Rendering|Material|SetScalarParameterValue _returnvalue "Invert HEight" 1.0 :!class /Script/Engine.MaterialInstanceDynamic)
        (else
          (Rendering|Material|SetScalarParameterValue _returnvalue "Invert Height" 0.0 :!class /Script/Engine.MaterialInstanceDynamic))))
    (:then_3
      (Rendering|Components|Decal|SetDecalMaterial (Variables|Default|GetDecal) _returnvalue))))