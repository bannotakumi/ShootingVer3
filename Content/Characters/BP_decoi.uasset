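; BP_decoi is a decoy that travels in a straight line along a direction set from a player rotation.
; SetPlayerRotate stores that rotation and rotates the current NowSpead movement vector by its roll and yaw, so repeated calls compound.
; Each Tick adds NowSpead to the location as a per-frame step without delta-time scaling and applies the stored roll and yaw to the actor.
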(event EventTick
  (params (DeltaSeconds :type Float%20%28single-precision%29))
  (bind _playerrotate (Variables|Default|GetPlayerRotate))
  ;[1 1 1] デコイの移動
  (Transformation|SetActorLocationAndRotation (+ (Transformation|GetActorLocation) (Variables|Default|GetNowSpead)) (Math|Rotator|MakeRotator (.roll _playerrotate) 0.0 (.yaw _playerrotate))))

(fn ConstructionScript)

(fn SetPlayerRotate
  (params (PlayerRotate :type Rotator))
  (bind _output_get (Variables|Default|SetPlayerRotate PlayerRotate))
  (bind _output_get_2 (Variables|Default|SetNewVar_0 _output_get))
  (Variables|Default|SetNowSpead (Math|Vector|RotateVector (Variables|Default|GetNowSpead) (Math|Rotator|MakeRotator (.roll _output_get_2) 0.0 (.yaw _output_get_2)))))