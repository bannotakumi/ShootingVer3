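; Pickable rifle actor for motion controller play, attached to the grabbing component on pickup and returned to physics on drop.
; Use and UnUse toggle a looping gunfire sound and firing flag, gated by remaining bullets.
; Magazine events refill or empty ammo with sounds, and dropping spawns an empty magazine at its socket.
; Bullet spawning, muzzle flash and ammo countdown are disconnected from the empty Tick; two-handed grip is unfinished.
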(event EventBeginPlay)

(event EventDropMagazine
  ;[1 1 1] マガジンを落とす
  (if (Variables|Default|GetmagazineChack)
    (Variables|Default|SetBullets 0)
    ;;[1 1 1] マガジンドロップ時のSE
    (Audio|SpawnSoundatLocation "/Game/Weapons/Sounds/AssultRifle/wav/sw_Wep_AR_Equip_02.sw_Wep_AR_Equip_02" (Transformation|GetActorLocation) "0, 0, 0" 1.0 1.0 0.0 0 0 false)
    ;;[1 1 1] マガジンの生成
    (Game|SpawnActorfromClass "/Game/FPS_Weapon_Bundle/Weapons/BP/MagazineEmpty.MagazineEmpty_C" (Transformation|GetSocketTransform (Variables|SkeletalMeshActor|GetSkeletalMeshComponent) "RifleMag" "RTS_World") "Undefined" 0 0)
    (Variables|Default|SetmagazineChack false)))

(event EventUse
  ;[1 1 1] 銃声
  (bind _bulletchack (CallFunction|MagazineCheck))
  (if _bulletchack
    (bind _returnvalue (Audio|SpawnSoundatLocation "/Game/Weapons/Sounds/AssultRifle/wav/sw_Wep_AR_Shoot_LP_01.sw_Wep_AR_Shoot_LP_01" (Transformation|GetActorLocation) "0, 0, 0" 1.0 1.0 0.0 0 0 false))
    (Variables|Default|SetUseSound _returnvalue)
    (Variables|Default|SetBulletShotCheck true)))

(event Collision|EventHit
  (params (MyComp :type Primitive%20Component%20Object%20Reference) (Other :type Actor%20Object%20Reference) (OtherComp :type Primitive%20Component%20Object%20Reference) (bSelfMoved :type Boolean) (HitLocation :type Vector :default "0, 0, 0") (HitNormal :type Vector :default "0, 0, 0") (NormalImpulse :type Vector :default "0, 0, 0") (Hit :type Hit%20Result%20Structure%20%28by%20ref%29))
  (Effects|SpawnEmitteratLocation "/Game/FXVarietyPack/Particles/P_ky_hit2.P_ky_hit2" HitLocation))

(event Collision|EventActorBeginOverlap
  (params (OtherActor :type Actor%20Object%20Reference))
  (Effects|SpawnEmitteratLocation "/Game/FXVarietyPack/Particles/P_ky_hit2.P_ky_hit2" (Transformation|GetActorLocation OtherActor)))

(event EventTick
  (params (DeltaSeconds :type Float%20%28single-precision%29)))

(event EventPickup
  (params (AttachTo :type Scene%20Component%20Object%20Reference) (SocketName :type Name :default "None"))
  (bind _skeletalmeshcomponent (Variables|SkeletalMeshActor|GetSkeletalMeshComponent))
  (Audio|SpawnSoundatLocation "/Game/Weapons/Sounds/AssultRifle/wav/sw_Wep_AR_Equip_01.sw_Wep_AR_Equip_01" (Transformation|GetActorLocation) "0, 0, 0" 1.0 1.0 0.0 0 0)
  (Physics|SetSimulatePhysics _skeletalmeshcomponent false)
  (Transformation|AttachComponentToComponent (Variables|Transformation|GetRootComponent) AttachTo SocketName "KeepWorld" "KeepWorld" "KeepWorld" false)
  (Transformation|SetRelativeLocationAndRotation _skeletalmeshcomponent "0.000000,-2.000000,-1.000000" "0, 0, 0" false false))

(event EventDrop
  (Physics|SetSimulatePhysics (Variables|SkeletalMeshActor|GetSkeletalMeshComponent) true)
  (Transformation|DetachFromActor "KeepWorld" "KeepWorld" "KeepWorld"))

(event EventUnUse
  (bind _usesound (Variables|Default|GetUseSound))
  ;[1 1 1] 銃を撃っていない状態
  (Utilities|IsValid _usesound
    (:Is%20Valid
      (Audio|Components|Audio|Stop _usesound)
      (Variables|Default|SetBulletShotCheck false))))

(event EventReleaseHand
  (params (AttachTo :type Boolean))
  ;[1 1 1] 両手持ち。未完成
)

(event EventSetHand
  (params (AttachTo :type Skeletal%20Mesh%20Component%20Object%20Reference))
  ;[1 1 1] 両手持ち。未完成
  (Transformation|AttachComponentToComponent AttachTo (Variables|Transformation|GetRootComponent) "SetHandSocket" "KeepWorld" "KeepWorld" "KeepWorld" false))

(event EventDetach
  ;[1 1 1] 手放す
  (Transformation|DetachFromActor "KeepWorld" "KeepWorld" "KeepWorld"))

(event EventAddMagazine
  ;[1 1 1] マガジンの追加
  (Development|PrintString "Hello")
  (if (not (Variables|Default|GetmagazineChack))
    (Variables|Default|SetBullets 30)
    ;;[1 1 1] マガジン装着時のSE
    (Audio|SpawnSoundatLocation "/Game/Weapons/Sounds/AssultRifle/wav/sw_Wep_Reload_AR.sw_Wep_Reload_AR" (Transformation|GetActorLocation) "0, 0, 0" 1.0 1.0 0.0 0 0 false)
    (Variables|Default|SetmagazineChack true)))

(fn ConstructionScript)

(fn GetPickGunRotation
  (return (Variables|Default|GetGun_Rotation)))

(fn ShotBullet
  (params (Bullet :type BP%20Bullet%20Object%20Reference))
  (Default|Rotation Bullet (Variables|Default|GetGun_Rotation)))

(fn MagazineCheck
  ;[1 1 1] 残弾があればtrue,なければfalse
  (return (> (Variables|Default|GetBullets) 0)))